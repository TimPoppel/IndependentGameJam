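; Base pet animal that tracks happiness, depression and energy, and dies when its energy runs out.
; Clicking its cube makes it happy and registers it with the player character.
; Each ThenextDay call either consumes happiness to lower depression, or depletes energy and raises depression, within a clamped range.
; Tick maps depression to the drain amount, prints debug values, and at zero energy swaps the animal for BP_Corpse after a delay.
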(event `self.Cube.OnClicked`
  (params (TouchedComponent :type "PrimitiveComponent Object Reference") (ButtonPressed :type "Key Structure"))
  (`self.SetHappy`)
  (bind _asbp_player_character (cast `/Game/Blueprints/BP_PlayerCharacter` (`GameplayStatics.GetPlayerCharacter` 0)))
  (`/Game/Blueprints/BP_PlayerCharacter.SetAnimal` _asbp_player_character self))

(event `The next Day`
  (bind _depressionstate (`self.DepressionState`))
  (if (`self.AmIhappy`)
    (`self.SetNotHappy`)
    (bind _result (`/Engine/EditorBlueprintResources/StandardMacros.DecrementInt` _depressionstate)
      (:`  `
        (if (<= _result 0)
          (set `self.DepressionState` 0)
          (else
            (set `self.DepressionState` _result)))))
    (else
      (`self.DepleteEnergy` (`self.Energydeplete`))
      (bind _result_2 (`/Engine/EditorBlueprintResources/StandardMacros.IncrementInt` _depressionstate)
        (:`  `
          (if (>= _result_2 3)
            (set `self.DepressionState` 3)
            (else
              (set `self.DepressionState` _result_2))))))))

(event `SetHappy`
  (set `self.AmIhappy` true))

(event `SetNotHappy`
  (set `self.AmIhappy` false))

(event `self.ReceiveBeginPlay`
  (set `self.CurrentEnergy` (`self.TotalEnergy`)))

(event `self.ReceiveTick`
  (params (DeltaSeconds :type "Float (single-precision)"))
  (bind _depressionstate (`self.DepressionState`))
  (if (== _depressionstate 0)
    (set `self.Energydeplete` 0.0)
    (elif (== _depressionstate 1)
      (set `self.Energydeplete` 1.0)
      (elif (== _depressionstate 2)
        (set `self.Energydeplete` 2.0)
        (elif (>= _depressionstate 3)
          (set `self.Energydeplete` 3.0)))))
  (if (<= (`self.CurrentEnergy`) 0.0)
    (`KismetSystemLibrary.Delay` 2.0)
    (`|SpawnActorFromClass` "/Game/Blueprints/Pets/BP_Corpse.BP_Corpse_C" (`self.GetTransform`) "Undefined" "OverrideRootScale" null null)
    (`self.K2_DestroyActor`)
    (else
      (`KismetSystemLibrary.PrintString` (`KismetStringLibrary.Conv_DoubleToString` (`self.CurrentEnergy`)))
      (`KismetSystemLibrary.PrintString` (`KismetStringLibrary.Conv_IntToString` (`self.DepressionState`))))))

(fn `DepleteEnergy`
  (params (Amount :type "Float (double-precision)"))
  (bind _returnvalue (- (`self.CurrentEnergy`) Amount))
  (if (<= _returnvalue 0.0)
    (set `self.CurrentEnergy` 0.0)
    (else
      (set `self.CurrentEnergy` _returnvalue))))

(fn `IncreaseEnergy`
  (params (Amount :type "Float (double-precision)"))
  (bind _returnvalue (+ (`self.CurrentEnergy`) Amount))
  (if (<= _returnvalue 0.0)
    (set `self.CurrentEnergy` 0.0)
    (else
      (set `self.CurrentEnergy` _returnvalue))))

(fn `UserConstructionScript`)