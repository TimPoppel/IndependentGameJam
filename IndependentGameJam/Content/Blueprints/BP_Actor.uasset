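; BP_Actor is a test actor that drives the BP_Dialogue widget with sample conversation lines.
; On BeginPlay it creates and displays the widget, records lines for speaker Tutel, some with answer options, then starts playback with the string "Tutel1".
; The ContinueDialogue input calls PlayDialogue again once the widget reports DialogueFinished.
; A Tutel1 event matching that string only prints a debug message.
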(event `self.ReceiveBeginPlay`
  (bind _returnvalue (`|CreateWidget` "/Game/Blueprints/Dialogue/BP_Dialogue.BP_Dialogue_C"))
  (set `self.Widget` _returnvalue)
  (`UserWidget.AddToViewport` _returnvalue 0)
  (`/Game/Blueprints/Dialogue/BP_Dialogue.Record Dialogue` :`self` _returnvalue :`Name` "Tutel" :`Dialogue` "Hello Jelle")
  (`/Game/Blueprints/Dialogue/BP_Dialogue.Record Dialogue` :`self` _returnvalue :`Name` "Tutel" :`Dialogue` "You are cringae" :`OptionAmount` 2 :`OptionText1` "1" :`OptionText2` "2")
  (`/Game/Blueprints/Dialogue/BP_Dialogue.Record Dialogue` :`self` _returnvalue :`Name` "Tutel" :`Dialogue` "Is roel also cringae? We had to expand this text for testing purposes so that we could see if it would work. Is roel also cringae? We had to expand this text for testing purposes so that we could see if it would work." :`OptionAmount` 3 :`OptionText1` "Yes" :`OptionText2` "No" :`OptionText3` "Monkey")
  (`/Game/Blueprints/Dialogue/BP_Dialogue.Play Dialogue` _returnvalue "Tutel1"))

(event `Tutel1`
  (`KismetSystemLibrary.PrintString` "Tutel1 is working" true true (struct :`R` 1.0 :`G` 0.02213 :`A` 1.0) 5.0))

(event `InputAction|ContinueDialogue`
  (params (Key :type "Key Structure"))
  (bind _widget (`self.Widget`))
  (:`Pressed`
    (if (`/Game/Blueprints/Dialogue/BP_Dialogue.DialogueFinished` _widget)
      (`/Game/Blueprints/Dialogue/BP_Dialogue.Play Dialogue` _widget ""))))

(fn `UserConstructionScript`)