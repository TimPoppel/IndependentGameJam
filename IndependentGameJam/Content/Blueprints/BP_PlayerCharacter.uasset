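; Player character that tracks an energy budget and drives the day cycle, with the mouse cursor shown.
; Tick ends the day at zero energy (key 0 forces it), calling TheNextDay on every BP_BaseAnimal, refilling energy and playing darkness, bedtime and delayed next-day widgets.
; Energy helpers only clamp at zero.
; P queues hardcoded test dialogue in BP_Dialogue, ContinueDialogue advances finished lines, and SetAnimal stores an animal reference.
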(event `self.ReceiveBeginPlay`
  (set `PlayerController.bShowMouseCursor` true (`GameplayStatics.GetPlayerController` 0))
  (bind _output_get (set `self.CurrentEnergy` (`self.TotalEnergy`)))
  (`KismetSystemLibrary.PrintString` (`KismetStringLibrary.Conv_DoubleToString` _output_get)))

(event `Key|P`
  (params (Key :type "Key Structure"))
  (:`Pressed`
    (bind _returnvalue (`|CreateWidget` "/Game/Blueprints/Dialogue/BP_Dialogue.BP_Dialogue_C"))
    (bind _output_get (set `self.Widget` _returnvalue))
    (`UserWidget.AddToViewport` _output_get 0)
    (`/Game/Blueprints/Dialogue/BP_Dialogue.Record Dialogue` (`self.Widget`) "Tutel" (struct :`R` 1.0 :`G` 0.904337 :`A` 1.0) "Hello Jelle" (struct :`R` 1.0 :`G` 1.0 :`B` 1.0 :`A` 1.0) 0 "" "" "")
    (`/Game/Blueprints/Dialogue/BP_Dialogue.Record Dialogue` (`self.Widget`) "Tutel" (struct :`R` 1.0 :`G` 0.404099 :`A` 1.0) "You are cringae" (struct :`R` 0.507324 :`G` 0.889569 :`B` 1.0 :`A` 1.0) 2 "1" "2" "")
    (`/Game/Blueprints/Dialogue/BP_Dialogue.Record Dialogue` (`self.Widget`) "Tutel" (struct :`R` 1.0 :`B` 0.042943 :`A` 1.0) "Is roel also cringae? We had to expand this text for testing purposes so that we could see if it would work. Is roel also cringae? We had to expand this text for testing purposes so that we could see if it would work." (struct :`R` 0.357114 :`G` 0.468546 :`B` 1.0 :`A` 1.0) 3 "Yes" "No" "Monkey")
    (`/Game/Blueprints/Dialogue/BP_Dialogue.Play Dialogue` (`self.Widget`) "Tutel1")))

(event `self.ReceiveTick`
  (params (DeltaSeconds :type "Float (single-precision)"))
  (if (<= (`self.CurrentEnergy`) 0.0)
    (`self.TriggerEndOfDay`)))

(event `TriggerEndOfDay`
  (bind _outactors (`GameplayStatics.GetAllActorsOfClass` "/Game/Blueprints/Pets/BP_BaseAnimal.BP_BaseAnimal_C"))
  (for _array_element _outactors
    (`/Game/Blueprints/Pets/BP_BaseAnimal.The next Day` _array_element))
  (set `self.CurrentEnergy` (`self.TotalEnergy`))
  (`self.TriggerTheEverLastingDarkness`)
  (`self.TriggerTimeToSleepWidget`)
  (`KismetSystemLibrary.Delay` 5.0)
  (`self.TriggerTheNextDayWidget`))

(event `Key|Zero`
  (params (Key :type "Key Structure"))
  (:`Pressed`
    (`self.TriggerEndOfDay`)))

(event `Tutel1`
  (`KismetSystemLibrary.PrintString` "Tutel1 is working" true true (struct :`R` 1.0 :`G` 0.02213 :`A` 1.0) 5.0))

(event `InputAction|ContinueDialogue`
  (params (Key :type "Key Structure"))
  (bind _widget (`self.Widget`))
  (:`Pressed`
    (`/Engine/EditorBlueprintResources/StandardMacros.IsValid` _widget
      (:`Is Valid`
        (if (`/Game/Blueprints/Dialogue/BP_Dialogue.DialogueFinished` _widget)
          (`/Game/Blueprints/Dialogue/BP_Dialogue.Play Dialogue` _widget ""))))))

(event `SetAnimal`
  (params (Animal :type "/Game/Blueprints/Pets/BP_BaseAnimal Object Reference"))
  (bind _output_get (set `self.WhatAnimalref` Animal))
  (`KismetSystemLibrary.PrintString` (`KismetSystemLibrary.GetDisplayName` _output_get)))

(fn `DecreaseEnergy`
  (params (Amount :type "Float (double-precision)"))
  (bind _returnvalue (- (`self.CurrentEnergy`) Amount))
  (if (<= _returnvalue 0.0)
    (set `self.CurrentEnergy` 0.0)
    (else
      (set `self.CurrentEnergy` _returnvalue))))

(fn `IncreaseEnergy`
  (params (Amount :type "Float (double-precision)"))
  (bind _returnvalue (+ (`self.CurrentEnergy`) Amount))
  (if (< _returnvalue 0.0)
    (set `self.CurrentEnergy` 0.0)
    (else
      (set `self.CurrentEnergy` _returnvalue))))

(fn `TriggerTheEverLastingDarkness`
  (bind _returnvalue (`|CreateWidget` "/Game/End_Of_The_Day/TheEverLastingDarkness.TheEverLastingDarkness_C"))
  (`UserWidget.AddToViewport` _returnvalue 0)
  (`UserWidget.PlayAnimation` _returnvalue (`/Game/End_Of_The_Day/TheEverLastingDarkness.TheEverLastingDarkness` _returnvalue) 0.0 1 "Forward" 1.0 false))

(fn `TriggerTheNextDayWidget`
  (bind _returnvalue (`|CreateWidget` "/Game/End_Of_The_Day/TheNextDay.TheNextDay_C"))
  (`UserWidget.AddToViewport` _returnvalue 0)
  (`UserWidget.PlayAnimation` _returnvalue (`/Game/End_Of_The_Day/TheNextDay.MoveAndFadeBorders` _returnvalue) 0.0 1 "Forward" 1.0 false)
  (`UserWidget.PlayAnimation` _returnvalue (`/Game/End_Of_The_Day/TheNextDay.MoveAndFadeText` _returnvalue) 0.0 1 "Forward" 1.0 false))

(fn `TriggerTimeToSleepWidget`
  (bind _returnvalue (`|CreateWidget` "/Game/End_Of_The_Day/Time_for_bed.Time_for_bed_C"))
  (`UserWidget.AddToViewport` _returnvalue 0)
  (`UserWidget.PlayAnimation` _returnvalue (`/Game/End_Of_The_Day/Time_for_bed.MoveAndFadeBorders` _returnvalue) 0.0 1 "Forward" 1.0 false)
  (`UserWidget.PlayAnimation` _returnvalue (`/Game/End_Of_The_Day/Time_for_bed.MoveAndFadeText` _returnvalue) 0.0 1 "Forward" 1.0 false)
  (`UserWidget.PlayAnimation` _returnvalue (`/Game/End_Of_The_Day/Time_for_bed.TheEverLastingDarkness` _returnvalue) 0.0 1 "Forward" 1.0 false))

(fn `UserConstructionScript`)