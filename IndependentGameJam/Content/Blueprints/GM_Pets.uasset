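; GM_Pets is a Blueprint, likely the game mode, that picks the player's ending from the fate of four pets: dog, cat, turtle and parrot.
; Each Tick checks flags: all dead without Rockdidit set calls EndingScene1 on BP_PlayerCharacter, while all friended calls FriendEnding.
; A shared Endingscene1triggered flag lets only one ending fire.
; Allenemiesdied is empty, and an unconnected energy-refill and next-day widget chain never runs.
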(event `self.ReceiveTick`
  (params (DeltaSeconds :type "Float (single-precision)"))
  (`|ExecutionSequence`
    (:`then_0`
      (if (`self.Dogdied`)
        (if (`self.Catdied`)
          (if (`self.Turtledied`)
            (if (`self.Parrotdied`)
              (if (`self.Rockdidit`)
                _
                (elif (not (`self.endingscene1triggered`))
                  (bind _asbp_player_character (cast `/Game/Blueprints/BP_PlayerCharacter` (`GameplayStatics.GetPlayerCharacter` 0)))
                  (`/Game/Blueprints/BP_PlayerCharacter.EndingScene1` _asbp_player_character)
                  (set `self.endingscene1triggered` true))))))))
    (:`then_1`
      (if (`self.DogFriend`)
        (if (`self.CatFriend`)
          (if (`self.TurtleFriend`)
            (if (`self.ParrotFriend`)
              (if (not (`self.endingscene1triggered`))
                (bind _asbp_player_character_2 (cast `/Game/Blueprints/BP_PlayerCharacter` (`GameplayStatics.GetPlayerCharacter` 0)))
                (`/Game/Blueprints/BP_PlayerCharacter.FriendEnding` _asbp_player_character_2)
                (set `self.endingscene1triggered` true)))))))))

(event `All enemies died`)

(fn `UserConstructionScript`)